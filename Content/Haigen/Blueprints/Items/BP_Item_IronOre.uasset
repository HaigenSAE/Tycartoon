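; Iron ore item Blueprint that turns into an iron bar when upgraded.
; Its Upgrade override calls the parent version, spawns BP_Item_IronBar slightly above the ore with the same rotation and scale, then destroys the ore.
; The event graph holds only disabled placeholder events, and the construction script just calls its parent.
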(fn `Upgrade`
  (bind (_returnvalue_location _returnvalue_rotation _returnvalue_scale) (`KismetMathLibrary.BreakTransform` (`self.GetTransform`)))
  (`parent.Upgrade`)
  (`|SpawnActorFromClass` "/Game/Haigen/Blueprints/Items/BP_Item_IronBar.BP_Item_IronBar_C" (`KismetMathLibrary.MakeTransform` (+ (0.0 0.0 5.0) _returnvalue_location) _returnvalue_rotation _returnvalue_scale) "Undefined" "OverrideRootScale" null null)
  (`self.K2_DestroyActor`))

(fn `UserConstructionScript`
  (`parent.UserConstructionScript`))