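; Spline-based conveyor belt that carries overlapping tycoon items and player characters along its path.
; The construction script builds two spline meshes per spline segment, one kept for overlap detection and one as a mesh.
; A fast looping timer offsets each overlapping actor along the closest spline direction, rotated to world space and scaled by MoveSpeed.
; A per-pass MovedActors list keeps actors spanning several segments from moving twice.
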(event `self.ReceiveBeginPlay`
  (`KismetSystemLibrary.K2_SetTimerDelegate` (delegate `MoveObjects`) 0.01 true))

(event `MoveObjects`
  (set `self.MovedActors` (`|MakeArray` self :!type "Actor Object Reference"))
  (for _array_element (`self.OverlapComponents`)
    (for _array_element_2 (`PrimitiveComponent.GetOverlappingActors` _array_element "/Game/Haigen/Blueprints/Items/BP_TycoonItem.BP_TycoonItem_C")
      (`self.MoveActors` _array_element_2))
    (for _array_element_3 (`PrimitiveComponent.GetOverlappingActors` _array_element "/Game/Haigen/Blueprints/Character/BP_TycoonPlayerCharacter.BP_TycoonPlayerCharacter_C")
      (`self.MoveActors` _array_element_3))))

(fn `MoveActors`
  (params (InputPin :type "Actor Object Reference"))
  (if (== (`KismetArrayLibrary.Array_Find` (`self.MovedActors`) InputPin) -1)
    (`self.K2_AddActorWorldOffset` InputPin (`KismetMathLibrary.GreaterGreater_VectorRotator` (* (`SplineComponent.FindDirectionClosestToWorldLocation` (`self.Spline`) (`self.K2_GetActorLocation` InputPin) "Local") (`self.moveSpeed`)) (`SceneComponent.K2_GetComponentRotation` (`self.DefaultSceneRoot`))) false false)
    (`KismetArrayLibrary.Array_Add` (`self.MovedActors`) InputPin)))

(fn `UserConstructionScript`
  (bind _spline (`self.Spline`))
  (for _index (range (+ (- (`SplineComponent.GetNumberOfSplinePoints` _spline) 2) 1))
    (bind _returnvalue (`AddComponent|NODE_AddSplineMeshComponent-0`))
    (`KismetArrayLibrary.Array_Add` (`self.OverlapComponents`) _returnvalue)
    (bind (_location _tangent) (`SplineComponent.GetLocationAndTangentAtSplinePoint` _spline _index "Local"))
    (bind (_location_2 _tangent_2) (`SplineComponent.GetLocationAndTangentAtSplinePoint` _spline (+ _index 1) "Local"))
    (`SplineMeshComponent.SetStartAndEnd` _returnvalue _location _tangent _location_2 _tangent_2 true)
    (bind _returnvalue_2 (`AddComponent|NODE_AddSplineMeshComponent-1`))
    (`KismetArrayLibrary.Array_Add` (`self.MeshComponents`) _returnvalue_2)
    (`SplineMeshComponent.SetStartAndEnd` _returnvalue_2 _location _tangent _location_2 _tangent_2 true)))