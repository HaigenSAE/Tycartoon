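; BP_ProductionBuilding is a building that periodically produces iron ore items in the world.
; One second after BeginPlay it starts a looping timer at the ProductionSpeed interval and stores the handle in Timer.
; Each tick of that timer spawns a quarter-scale BP_Item_IronOre actor at the DispenserLoc component's world location.
; The item class is hardcoded, and Tick and overlap events are unused.
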(event `self.ReceiveBeginPlay`
  (`parent.ReceiveBeginPlay`)
  (`KismetSystemLibrary.Delay` 1.0)
  (bind _returnvalue (`KismetSystemLibrary.K2_SetTimerDelegate` (delegate `ProduceItem`) (`self.productionSpeed`) true))
  (set `self.Timer` _returnvalue))

(event `ProduceItem`
  (`|SpawnActorFromClass` "/Game/Haigen/Blueprints/Items/BP_Item_IronOre.BP_Item_IronOre_C" (`KismetMathLibrary.MakeTransform` (`SceneComponent.K2_GetComponentLocation` (`self.DispenserLoc`)) (struct) (0.25 0.25 0.25)) "Undefined" "OverrideRootScale" null null))

(fn `UserConstructionScript`
  (`parent.UserConstructionScript`))